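; Breakable jar (jarrón) that spills coins when the Samurai hits it, then sinks away.
; A hit on Jarron_DM spawns Monedas actors at random XY points within a Box, slightly above its center.
; It also enables physics and applies high radial damage at the impact point, credited to the Samurai.
; After a delay, a timeline moves the mesh downward, lerping from its current location on each update.
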(event `self.ReceiveBeginPlay`)

(event `self.ReceiveTick`
  (params (DeltaSeconds :type "Float (single-precision)")))

(event `self.jarron_DM.OnComponentHit`
  (params (HitComponent :type "PrimitiveComponent Object Reference") (OtherActor :type "Actor Object Reference") (OtherComp :type "PrimitiveComponent Object Reference") (NormalImpulse :type "Vector Structure") (Hit :type "HitResult Structure (by ref)"))
  (bind _jarron_dm (`self.jarron_DM`))
  (bind (_returnvalue_x _returnvalue_y _returnvalue_z) (`KismetMathLibrary.BreakVector` (`SceneComponent.K2_GetComponentLocation` _jarron_dm)))
  (bind _assamurai (cast `/Game/Personajes/Samurai` OtherActor))
  (`self.SpawnMonedas`)
  (`PrimitiveComponent.SetSimulatePhysics` (`self.jarron_DM`) true)
  (`GameplayStatics.ApplyRadialDamage` :`BaseDamage` 1000.0 :`Origin` Hit_ImpactPoint :`DamageRadius` 100.0 :`DamageCauser` _assamurai :`bDoFullDamage` true)
  (`KismetSystemLibrary.Delay` 3.0)
  (bind (_direction _newtrack_0) (`Timeline|Timeline_0`)
    (:`Update`
      (`SceneComponent.K2_SetWorldLocation` _jarron_dm (`KismetMathLibrary.VLerp` (`KismetMathLibrary.MakeVector` _returnvalue_x _returnvalue_y _returnvalue_z) (`KismetMathLibrary.MakeVector` _returnvalue_x _returnvalue_y (- _returnvalue_z 200.0)) _newtrack_0) false false))))

(fn `SpawnMonedas`
  (bind _box (`self.Box`))
  (bind _returnvalue (`SceneComponent.K2_GetComponentLocation` _box))
  (bind (_returnvalue_x _returnvalue_y) (`KismetMathLibrary.BreakVector` (`KismetMathLibrary.RandomPointInBoundingBox` _returnvalue (`BoxComponent.BoxExtent` _box))))
  (for _ (range 6)
    (`|SpawnActorFromClass` "/Game/Actores/Monedas.Monedas_C" (`KismetMathLibrary.Conv_VectorToTransform` (`KismetMathLibrary.MakeVector` _returnvalue_x _returnvalue_y (+ (.z _returnvalue) 50.0))) "Undefined" "OverrideRootScale" null null)))

(fn `UserConstructionScript`)